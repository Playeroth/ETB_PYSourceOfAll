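; Peaceful mode mod actor that removes or neutralizes entities and hazards, with handling chosen by level name.
; BeginPlay handles some level-specific hazards, while Delays on Tick throttle a repeating sweep and later hazard fixes.
; The sweep gathers non-player Characters for EntityRemoval, which destroys them by default and also clears spawn triggers on certain levels.
; Exception levels spare certain classes or disable overlaps on "KillPlayer" components, sometimes freezing movement.
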(event EventBeginPlay
  (bind _returnvalue (Game|GetCurrentLevelName true))
  (switch string _returnvalue
    (:Level07
      (bind _returnvalue_2 (Actor|GetActorOfClass "/Game/Entity/BoneThief/BP_BoneThief.BP_BoneThief_C"))
      (Actor|DestroyActor _returnvalue_2))
    (:Level188_Expanded
      (bind _outactors (Actor|GetAllActorsOfClass "/Game/Entity/Windows/BP_Windows.BP_Windows_C"))
      (Actor|DestroyActor _outactors))
    (:Grassrooms_Expanded
      (bind _outactors_2 (Actor|GetAllActorsOfClass "/Game/Grassrooms/BP_VinesDisabled_Zone.BP_VinesDisabled_Zone_C"))
      (for _array_element _outactors_2
        (Actor|DestroyActor _array_element))
      (Game|SpawnActorfromClass "/Game/Grassrooms/BP_VinesDisabled_Zone.BP_VinesDisabled_Zone_C" (Math|Transform|MakeTransform "0, 0, 0" "0, 0, 0" "99999.000000,99999.000000,99999.000000") "AlwaysSpawn" 0 0))))

(event EventTick
  (params (DeltaSeconds :type Float%20%28single-precision%29))
  ;[1 1 1 1 16] Initial Operation
  (Utilities|FlowControl|Sequence
    (:then_0
      (Utilities|FlowControl|Delay 1.0)
      ;[1 1 1 1 16] Gets all Entities And then remove
      (Utilities|GetandSetEntities))
    (:then_1
      (Utilities|FlowControl|Delay 3.0)
      (bind _returnvalue (Game|GetCurrentLevelName true))
      (switch string _returnvalue
        (:Level188_Expanded
          (bind _outactors (Actor|GetAllActorsOfClass "/Game/Entity/Windows/BP_Windows.BP_Windows_C"))
          (for _array_element _outactors
            (Variables|/Script/Engine.PrimitiveComponent|SetbGenerateOverlapEvents (Actor|GetComponentbyClass _array_element "/Script/Engine.CapsuleComponent") false)))
        (:Poolrooms_Expanded
          (bind _outactors_2 (Actor|GetAllActorsOfClass "/Game/Entity/HydroPlague/BP_HydroPlague.BP_HydroPlague_C"))
          (Actor|DestroyActor _outactors_2))))))

(fn ConstructionScript
  (|CallParentFunction))

(fn ModButtonWasPressed
  (params (FunctionIndex :type Integer))
  (switch int FunctionIndex))

(fn Testing)